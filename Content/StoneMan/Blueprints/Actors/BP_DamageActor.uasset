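; BP_DamageActor is a placeable hazard that periodically deals radial damage around its location.
; On BeginPlay a looping timer calls MakeDamage at DamageFrequency, applying radial damage with configurable amount, radius and full-damage flag, using Pawn as the damage prevention channel.
; The construction script sizes the DamageArea sphere to DamageRadius, while Tick draws a red debug sphere showing the damage range.
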(event EventBeginPlay
  (Utilities|Time|SetTimerbyFunctionName 0 "MakeDamage" (Variables|Default|GetDamageFrequency) true))

(event Collision|EventActorBeginOverlap
  (params (OtherActor :type Actor%20Object%20Reference)))

(event EventTick
  (params (DeltaSeconds :type Float%20%28single-precision%29))
  (Rendering|Debug|DrawDebugSphere (Transformation|GetActorLocation) (Variables|Default|GetDamageRadius) 24 "(R=1.000000,G=0.000000,B=0.000000,A=1.000000)" 0.0 1.5))

(fn ConstructionScript
  (Components|Sphere|SetSphereRadius (Variables|Default|GetDamageArea) (Variables|Default|GetDamageRadius) false))

(fn MakeDamage
  (Game|Damage|ApplyRadialDamage (Variables|Default|GetDamageAmount) (Transformation|GetActorLocation) (Variables|Default|GetDamageRadius) 0 0 0 0 (Variables|Default|GetDoFullDamage) "ECC_Pawn"))